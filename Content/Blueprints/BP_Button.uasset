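; BP_Button is a pressable rock button that temporarily hides a video screen when an overlapping actor, intended as the player's hand, touches it.
; On actor overlap it confirms contact with RockButton, lowers it and hides VideoScreen, then restores both after a fixed delay.
; The IsBranchEnded flag gates the sequence so further overlaps cannot retrigger or re-offset the button until the reset completes.
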(event `self.ReceiveBeginPlay`)

(event `self.ReceiveActorBeginOverlap`
  (params (OtherActor :type "Actor Object Reference"))
  (bind _rockbutton (`self.RockButton`))
  (bind _videoscreen (`self.VideoScreen`))
  (bind _output_get (set `self.IsPressed` (`PrimitiveComponent.IsOverlappingActor` _rockbutton OtherActor)))
  (if (and _output_get (`self.IsBranchEnded`))
    (set `self.IsBranchEnded` false)
    (`SceneComponent.K2_AddLocalOffset` _rockbutton (0.0 0.0 -10.0) false false) ; move cube to pressed position
    (`SceneComponent.SetVisibility` _videoscreen false false) ; Makes the video screen disappear
    (`KismetSystemLibrary.Delay` 6.0)
    (`SceneComponent.K2_AddLocalOffset` _rockbutton (0.0 0.0 10.0) false false) ; move cube to not pressed position
    (`SceneComponent.SetVisibility` _videoscreen true false) ; makes the video screen reappear
    (set `self.IsBranchEnded` true) ; sets true when finsihed the branch
  ))

(fn `UserConstructionScript`)